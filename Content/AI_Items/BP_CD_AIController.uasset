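; AI controller for BP_CombatBot that runs the CD_AICombatBot behavior tree and marches the bot along a spline lane.
; Shortly after BeginPlay, it assigns the nearest spline actor and caches its points, reversing them for bots not on Team1.
; GoingNextPoint chains AIMoveTo calls with slight random offsets, setting rotation from the spline, negated for the opposing team.
; Keepmoving resumes movement after victory, while the weapon, team and data getters are empty stubs.
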(event `self.ReceivePossess`
  (params (PossessedPawn :type "Pawn Object Reference"))
  (`self.RunBehaviorTree` "/Game/AI_Items/CD_AICombatBot.CD_AICombatBot"))

(event `self.ReceiveBeginPlay`
  (bind _pointsspline (`self.PointsSpline`))
  ;[1 1 1] TakeNearestSplinefor movement
  (`KismetSystemLibrary.Delay` 0.2)
  (bind _outactors (`GameplayStatics.GetAllActorsOfClass` "/Game/Player/BP_CD_SplineMeshActor.BP_CD_SplineMeshActor_C"))
  (bind _asbp_cd_spline_mesh_actor (cast `/Game/Player/BP_CD_SplineMeshActor` (`.ReturnValue` (`GameplayStatics.FindNearestActor` (`self.K2_GetActorLocation` (`self.K2_GetPawn`)) _outactors))))
  (bind _output_get (set `self.CurrentSpline` (`/Game/Player/BP_CD_SplineMeshActor.Spline` _asbp_cd_spline_mesh_actor)))
  (bind _asbp_combat_bot (cast `/Game/Items/BP_CombatBot` (`self.K2_GetPawn`)))
  (set `/Game/Items/BP_CombatBot.Spline Ref` _asbp_cd_spline_mesh_actor _asbp_combat_bot)
  (`self.CreatePointsMovement` _output_get
    (:`Completed`
      ;[1 1 1] MovementCombatBot
      (bind _returnvalue (message `CD_GameCreature.GetTeam` (`self.K2_GetPawn`)))
      (if (not (`|EnumEquality` _returnvalue "Team1"))
        (`KismetArrayLibrary.Array_Reverse` _pointsspline))
      (`KismetArrayLibrary.Array_Remove` _pointsspline)
      (`self.GoingNextPoint`))))

(event `Keep moving`
  ;[1 1 1] MovementCombatBot
  ;;[1 1 1] MoveAfterVictory
  (`self.GoingNextPoint`))

(fn `GetDataCombatBot`
  (returns (ReturnValue :type "CD_DataCombatBot Structure"))
  (return))

(fn `GetTeam`
  (returns (ReturnValue :type "ECD_Team Enum"))
  (return "None"))

(fn `GetWeaponInfo`
  (returns (ReturnValue :type "CD_WeaponType Structure"))
  (return))

(fn `UserConstructionScript`)
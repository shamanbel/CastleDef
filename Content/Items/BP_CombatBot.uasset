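; Combat bot pawn that travels under AI control and automatically fights other-team actors entering its interaction sphere.
; On BeginPlay it hooks up its health bar and loads speed, weapon and reload time from bot and weapon databases.
; An enemy overlap stops movement, links combat anim layers and starts an attack loop driven by ReloadComponent, firing projectiles or applying direct damage.
; When a target becomes invalid, it switches to another or tells the AI controller to keep moving.
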(event `self.ReceiveBeginPlay`
  (bind _reloadcomponent (`self.ReloadComponent`))
  ;[1 1 1] Set HealthBar for each combat bot
  (`parent.ReceiveBeginPlay`)
  (bind _asw_health_bar_combat_bot (cast `/Game/HUD/W_Item/W_HealthBarCombatBot` (`WidgetComponent.GetUserWidgetObject` (`self.HealthBar`))))
  (set `/Game/HUD/W_Item/W_HealthBarCombatBot.CombatBotRef` self _asw_health_bar_combat_bot)
  (`KismetSystemLibrary.Delay` 0.01)
  ;[1 1 1] Set Velocity &Weapon & Timer for reload
  (bind _returnvalue (`CD_CombatBotDataBase.GetDataByClassBP` (subsystem `CD_CombatBotDataBase`) (`self.BotID`)))
  (bind (_spawnactorclass _combatbot_id _weapon_id _typecombatbot _ratiocostcombatbot _velocitycombatbot) (break `CD_DataCombatBot` _returnvalue))
  (bind _returnvalue_2 (`CD_WeaponDatabase.GetDataByClassBP` (subsystem `CD_WeaponDatabase`) _weapon_id))
  (bind _output_get (set `self.WeaponCurrentID` _returnvalue_2))
  (set `FloatingPawnMovement.MaxSpeed` _velocitycombatbot (`self.FloatingPawnMovement`))
  (`ReloadComponent.SetReloadTime` _reloadcomponent (`.ReloadTime` (break `CD_WeaponType` _output_get)) false)
  (add `ReloadComponent.OnReloadFinished` _reloadcomponent (delegate `ApplyDamage11`)))

(event `ApplyDamage11`
  (bind _actorstarget (`self.ActorsTarget`))
  ;[1 1 1] Set Velocity &Weapon & Timer for reload
  (`/Engine/EditorBlueprintResources/StandardMacros.IsValid` (`self.DamagedActor`)
    (:`Is Valid`
      (`self.Apply Damage` (`.Damage` (break `CD_WeaponType` (stale `self.ReceiveBeginPlay` _output_get)))))
    (:`Is Not Valid`
      ;[1 1 1] Checkforfight
      (`SkeletalMeshComponent.UnlinkAnimClassLayers` (`self.SkeletalMesh`) (`self.ABPRef`))
      (`KismetArrayLibrary.Array_RemoveItem` _actorstarget (`self.DamagedActor`))
      (if (== (`KismetArrayLibrary.Array_Length` _actorstarget) 0)
        (bind _asbp_cd_aicontroller (cast `/Game/AI_Items/BP_CD_AIController` (`self.GetController`)))
        (`/Game/AI_Items/BP_CD_AIController.Keep moving` _asbp_cd_aicontroller)
        (else
          (set `self.DamagedActor` (`|GetArrayItem` _actorstarget))
          (`ReloadComponent.FinishReload` (`self.ReloadComponent`)))))))

(event `self.SphereInteraction.OnComponentBeginOverlap`
  (params (OverlappedComponent :type "PrimitiveComponent Object Reference") (OtherActor :type "Actor Object Reference") (OtherComp :type "PrimitiveComponent Object Reference") (OtherBodyIndex :type Integer) (bFromSweep :type Boolean) (SweepResult :type "HitResult Structure (by ref)"))
  ;[1 1 1] Begin fight
  ;;[1 1 1] For Init TeamCombatBot
  (`KismetSystemLibrary.Delay` 0.01)
  (bind _returnvalue (message `CD_GameCreature.GetTeam` OtherActor))
  (if (`|EnumInequality` (`self.TeamCombatBot`) _returnvalue)
    (set `self.DamagedActor` OtherActor)
    (`MovementComponent.StopMovementImmediately` (`self.FloatingPawnMovement`))
    (`KismetArrayLibrary.Array_Add` (`self.ActorsTarget`) (`self.DamagedActor`))
    (`SkeletalMeshComponent.LinkAnimClassLayers` (`self.SkeletalMesh`) (`self.ABPRef`))
    (`ReloadComponent.FinishReload` (`self.ReloadComponent`))))

(fn `Apply Damage`
  (params (BaseDamage :type "Float (double-precision)"))
  (if (`self.bIsShootingProjectile`)
    (`self.ShotProjectile`)
    (else
      (`GameplayStatics.ApplyDamage` (`self.DamagedActor`) BaseDamage null self)))
  (`ReloadComponent.StartReload` (`self.ReloadComponent`)))

(fn `GetTeam`
  (returns (ReturnValue :type "ECD_Team Enum"))
  (return (`self.TeamCombatBot`)))

(fn `UserConstructionScript`)
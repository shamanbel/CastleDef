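; BP_SpawnPlace is an actor marking a clickable location for spawning a combat bot.
; Its Place component starts hidden on BeginPlay and responds to clicks only while visible.
; A valid click stores the actor's location as SpawnPosition on BP_CD_GameMode, then calls SpawnCombatBot on BP_PlayerController for player 0.
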(event `self.ReceiveBeginPlay`
  (`SceneComponent.SetVisibility` (`self.  place`) false false))

(event `self.  place.OnClicked`
  (params (TouchedComponent :type "PrimitiveComponent Object Reference") (ButtonPressed :type "Key Structure"))
  (if (`SceneComponent.IsVisible` (`self.  place`))
    (bind _asbp_cd_game_mode (cast `/Game/Level/BP_CD_GameMode` (`GameplayStatics.GetGameMode`)))
    (set `/Game/Level/BP_CD_GameMode.SpawnPosition` (`self.K2_GetActorLocation`) _asbp_cd_game_mode)
    (bind _asbp_player_controller (cast `/Game/Player/BP_PlayerController` (`GameplayStatics.GetPlayerController` 0)))
    (`/Game/Player/BP_PlayerController.SpawnCombatBot` _asbp_player_controller)))

(fn `UserConstructionScript`)
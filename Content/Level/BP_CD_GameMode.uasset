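; Game mode that spawns combat bots for teams.
; On BeginPlay it scans spawn place actors and alternately stores Team2 locations into two AI spawn positions.
; SpawnCombatBot looks up the bot class by ID in the database, spawns it at a team-based location (random between the two for AI), sets ID and team, fires the spawn notification and returns success.
; An unconnected older spawn path with weapon and kill-reward setup remains.
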(event `self.ReceiveBeginPlay`
  (bind _outactors (`GameplayStatics.GetAllActorsOfClass` "/Game/Items/BP_SpawnPlace.BP_SpawnPlace_C"))
  (for _array_element _outactors
    (if (`|EnumEquality` (`/Game/Items/BP_SpawnPlace.TeamSpawnPlace` _array_element) "Team2")
      (`/Engine/EditorBlueprintResources/StandardMacros.FlipFlop`
        (:`A`
          (bind _returnvalue (`self.K2_GetActorLocation` _array_element))
          (set `self.AISpawnPosition01` _returnvalue))
        (:`B`
          (set `self.AISpawnPosition02` _returnvalue))))))

(fn `Spawn Combat Bot`
  (params (IDCombatBot :type "CD_BaseCombatBotID Class Reference") (Team :type "ECD_Team Enum" :default "None"))
  (returns (Success :type Boolean))
  (locals (NewLocalVar_0 :type "Float (double-precision)" :default 0.0))
  (bind _returnvalue (`CD_CombatBotDataBase.GetDataByClassBP` (subsystem `CD_CombatBotDataBase`) IDCombatBot))
  (bind _returnvalue_2 (`|SpawnActorFromClass` (break `CD_DataCombatBot` _returnvalue) (`KismetMathLibrary.MakeTransform` (select `byte` Team :`0` (0.0 0.0 0.0) :`1` (`self.SpawnPosition`) :`2` (select `int` (`KismetMathLibrary.RandomIntegerInRange` 0 1) :`0` (`self.AISpawnPosition01`) :`1` (`self.AISpawnPosition02`)))) "AlwaysSpawn" "OverrideRootScale" null null))
  (bind _asbp_combat_bot (cast `/Game/Items/BP_CombatBot` _returnvalue_2)
    (:`then`
      (set `CD_CombatBot.BotID` IDCombatBot _asbp_combat_bot)
      (set `CD_CombatBot.TeamCombatBot` Team _asbp_combat_bot)
      (`self.OnCombatBotSpawn` _asbp_combat_bot)
      (return true))
    (:`CastFailed`
      (return false))))

(fn `UserConstructionScript`)
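; Player controller for a castle battle game that buys combat bots for both the player and the AI.
; On BeginPlay it caches both castles by team and shows the HUD in PlayLevel; pause input adds the pause menu and flip-flops game pause.
; Spawn functions deduct database-driven costs from the owning castle, then spawn through the GameMode.
; AI spawns roll cost and bot type separately, never reaching the vehicle option.
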(event `self.ReceiveBeginPlay`
  ;[1 1 1] Set ref
  (bind _outactors (`GameplayStatics.GetAllActorsOfClass` "/Game/Items/BP_BaseCastle.BP_BaseCastle_C"))
  (for _array_element _outactors
    (if (`|EnumEquality` (`CD_BaseCastle.TeamCastle` _array_element) "Team1")
      (set `self.CastleRef` _array_element)
      (else
        (set `self.AICastleRef` _array_element))))
  (bind _returnvalue (`GameplayStatics.GetCurrentLevelName` true))
  ;[1 1 1] PlayerWidget
  (if (`KismetStringLibrary.EqualEqual_StrStr` _returnvalue "PlayLevel")
    (`/Engine/EditorBlueprintResources/StandardMacros.IsValid` (`self.PlayerHUDRef`)
      (:`Is Valid`
        _)
      (:`Is Not Valid`
        (bind _returnvalue_2 (`|CreateWidget` "/Game/HUD/PlayerHUD.PlayerHUD_C"))
        (bind _output_get (set `self.PlayerHUDRef` _returnvalue_2))))
    (`UserWidget.AddToViewport` _output_get 0)))

(event `InputAction|PauseGame`
  (params (Key :type "Key Structure"))
  (:`Pressed`
    (`/Engine/EditorBlueprintResources/StandardMacros.IsValid` (`self.PauseMenuRef`)
      (:`Is Valid`
        _)
      (:`Is Not Valid`
        (bind _returnvalue (`|CreateWidget` "/Game/HUD/Menu/Pause.Pause_C"))
        (bind _output_get (set `self.PauseMenuRef` _returnvalue))))
    (`UserWidget.AddToViewport` _output_get 0)
    (`/Engine/EditorBlueprintResources/StandardMacros.FlipFlop`
      (:`A`
        (`GameplayStatics.SetGamePaused` true))
      (:`B`
        (`GameplayStatics.SetGamePaused` false)))))

(fn `SpawnAI_CombatBot`
  (returns (Succes :type Boolean))
  (bind _returnvalue (select `int` (`KismetMathLibrary.RandomIntegerInRange` 0 2) :`0` "/Game/Data/CombatBot_IDs/CombatBot_Artillery.CombatBot_Artillery_C" :`1` "/Game/Data/CombatBot_IDs/CombatBot_Melee.CombatBot_Melee_C" :`2` "/Game/Data/CombatBot_IDs/CombatBot_Range.CombatBot_Range_C" :`3` "/Game/Data/CombatBot_IDs/CombatBot_Vihicle.CombatBot_Vihicle_C" :!type "CD_BaseCombatBotID Class Reference"))
  (`/Engine/EditorBlueprintResources/StandardMacros.IsValid` (`self.AICastleRef`)
    (:`Is Valid`
      (bind _returnvalue_2 (`CD_CombatBotDataBase.GetDataByClassBP` (subsystem `CD_CombatBotDataBase`) _returnvalue))
      (bind _returnvalue_3 (`CD_BaseCastle.ChangeMoney` (`self.AICastleRef`) (* (* (`.RatioCostCombatBot` (break `CD_DataCombatBot` _returnvalue_2)) (`CD_DataAssetStartMatchSettings.BaseCostCombatBot` (`self.StartSet`))) -1.0)))
      (if _returnvalue_3
        (bind _asbp_cd_game_mode (cast `/Game/Level/BP_CD_GameMode` (`GameplayStatics.GetGameMode`)))
        (bind _success (`/Game/Level/BP_CD_GameMode.Spawn Combat Bot` _asbp_cd_game_mode _returnvalue "Team2"))
        (return _success)))))

(fn `SpawnCombatBot`
  (bind _in_id_combat_bot (`self.In Id Combat Bot`))
  (`/Engine/EditorBlueprintResources/StandardMacros.IsValid` (`self.CastleRef`)
    (:`Is Valid`
      (bind _returnvalue (`CD_CombatBotDataBase.GetDataByClassBP` (subsystem `CD_CombatBotDataBase`) _in_id_combat_bot))
      (bind _returnvalue_2 (`CD_BaseCastle.ChangeMoney` (`self.CastleRef`) (* (* (`.RatioCostCombatBot` (break `CD_DataCombatBot` _returnvalue)) (`CD_DataAssetStartMatchSettings.BaseCostCombatBot` (`self.startSet`))) -1.0)))
      (if _returnvalue_2
        (bind _asbp_cd_game_mode (cast `/Game/Level/BP_CD_GameMode` (`GameplayStatics.GetGameMode`)))
        (`/Game/Level/BP_CD_GameMode.Spawn Combat Bot` _asbp_cd_game_mode _in_id_combat_bot "Team1")))
    (:`Is Not Valid`
      (`KismetSystemLibrary.PrintString` "You Fail"))))

(fn `UserConstructionScript`)